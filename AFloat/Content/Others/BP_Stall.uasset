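; BP_Stall is a stall actor that keeps track of the BP_DefaultStaff actors placed inside its overlap area.
; On BeginPlay it gathers its ChildActorComponents into an Order array, which this graph does not use further.
; Begin and end overlap events add and remove those actors in the Staphs array without duplicates, printing a debug "put" or "remove" message.
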(event Collision|EventActorBeginOverlap
  (params (OtherActor :type Actor%20Object%20Reference))
  (bind _asbp_default_staff (Utilities|Casting|CastToBP_DefaultStaff OtherActor))
  (Utilities|Array|AddUnique (Variables|Default|GetStaphs) _asbp_default_staff)
  (Development|PrintString "put"))

(event EventTick
  (params (DeltaSeconds :type Float%20%28single-precision%29)))

(event EventBeginPlay
  (for _array_element (Actor|GetComponentsByClass "/Script/Engine.ChildActorComponent")
    (Utilities|Array|Add (Variables|Default|GetOrder) _array_element)))

(event Collision|EventActorEndOverlap
  (params (OtherActor :type Actor%20Object%20Reference))
  (bind _asbp_default_staff (Utilities|Casting|CastToBP_DefaultStaff OtherActor))
  (Utilities|Array|RemoveItem (Variables|Default|GetStaphs) _asbp_default_staff)
  (Development|PrintString "remove"))

(fn ConstructionScript)
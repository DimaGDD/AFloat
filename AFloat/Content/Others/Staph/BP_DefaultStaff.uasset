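; BP_DefaultStaff is a physical item with a price that drops when it takes hard impacts.
; On Hit, its component's speed times mass is checked against a threshold, then scaled into damage subtracted from Price.
; The actor is destroyed when Price runs out; otherwise a damage widget animates in, then reverses after a delay.
; Outline events toggle an overlay material on the mesh for highlighting.
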(event Collision|EventHit
  (params (MyComp :type Primitive%20Component%20Object%20Reference) (Other :type Actor%20Object%20Reference) (OtherComp :type Primitive%20Component%20Object%20Reference) (bSelfMoved :type Boolean) (HitLocation :type Vector :default "0, 0, 0") (HitNormal :type Vector :default "0, 0, 0") (NormalImpulse :type Vector :default "0, 0, 0") (Hit :type Hit%20Result%20Structure%20%28by%20ref%29))
  (Variables|Default|SetForce%20Hit (* (Math|Vector|VectorLength (Transformation|GetComponentVelocity MyComp)) (Physics|GetMass MyComp)))
  (if (> (Variables|Default|GetForce%20Hit) (Variables|Default|GetMin%20Damage%20Stage))
    (Variables|Default|SetDamage (Math|Float|Truncate (* (Variables|Default|GetForce%20Hit) 0.05)))
    (Variables|Default|SetPrice (- (Variables|Default|GetPrice) (Variables|Default|GetDamage)))
    (if (<= (Variables|Default|GetPrice) 0.0)
      (Actor|DestroyActor)
      (else
        (bind _returnvalue (UserInterface|CreateWidget "/Game/Others/Staph/UI_ProductDamage.UI_ProductDamage_C"))
        (Variables|Default|SetInteraction%20Widget _returnvalue)
        (Default|ChangeDamageText (Variables|Default|GetInteraction%20Widget) (Variables|Default|GetDamage))
        (UserInterface|SetWidget (Variables|Default|GetWidget) (Variables|Default|GetInteraction%20Widget))
        (Rendering|SetVisibility (Variables|Default|GetWidget) true false)
        (UserInterface|Animation|PlayAnimation (Variables|Default|GetInteraction%20Widget) (Variables|/Game/Others/Staph/UI_ProductDamage.UI_ProductDamage_C|GetDamage (Variables|Default|GetInteraction%20Widget)) 0.0 1 "Forward" 1.5 false)
        (Utilities|FlowControl|Delay 1.0)
        (UserInterface|Animation|PlayAnimation (Variables|Default|GetInteraction%20Widget) (Variables|/Game/Others/Staph/UI_ProductDamage.UI_ProductDamage_C|GetDamage (Variables|Default|GetInteraction%20Widget)) 0.0 1 "Reverse" 1.5 false)))))

(event EventOutlineEnable
  (Rendering|Material|SetOverlayMaterial (Variables|Default|GetStaticMesh) "/Game/Others/Staph/M_Outline_Inst.M_Outline_Inst" :!class /Script/Engine.MeshComponent))

(event EventOutlineDisable
  (Rendering|Material|SetOverlayMaterial (Variables|Default|GetStaticMesh) 0 :!class /Script/Engine.MeshComponent))

(fn ConstructionScript)
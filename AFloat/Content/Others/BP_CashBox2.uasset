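; Checkout counter where a customer NPC's products are scanned and paid for.
; When a product leaves the PaymentPIC zone and is in the reserved map of Slot1's NPC, it plays a beep, credits its price to the player and destroys the product.
; An emptied map sets the NPC's PaymentPass blackboard key.
; A cashier zone tracks player presence without gating payment, and only the first of three queue slots is served.
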(event OnComponentBeginOverlap(PlaceForKassir)
  (params (OverlappedComponent :type Primitive%20Component%20Object%20Reference) (OtherActor :type Actor%20Object%20Reference) (OtherComp :type Primitive%20Component%20Object%20Reference) (OtherBodyIndex :type Integer) (bFromSweep :type Boolean) (SweepResult :type Hit%20Result%20Structure%20%28by%20ref%29))
  (Utilities|Casting|CastToBP_MainCharacter OtherActor)
  (Variables|Default|SetPlayer%20on%20kassa true)
  (Development|PrintString "Player in kassa"))

(event OnComponentEndOverlap(PlaceForKassir)
  (params (OverlappedComponent :type Primitive%20Component%20Object%20Reference) (OtherActor :type Actor%20Object%20Reference) (OtherComp :type Primitive%20Component%20Object%20Reference) (OtherBodyIndex :type Integer))
  (Utilities|Casting|CastToBP_MainCharacter OtherActor)
  (Variables|Default|SetPlayer%20on%20kassa false)
  (Development|PrintString "Player not in kassa"))

(event OnComponentEndOverlap(PaymentPIC)
  (params (OverlappedComponent :type Primitive%20Component%20Object%20Reference) (OtherActor :type Actor%20Object%20Reference) (OtherComp :type Primitive%20Component%20Object%20Reference) (OtherBodyIndex :type Integer))
  (bind _asbp_default_staff (Utilities|Casting|CastToBP_DefaultStaff OtherActor))
  (Variables|Default|SetProduct%20For%20PIC _asbp_default_staff)
  (bind _asbp_order_slot (Utilities|Casting|CastToBP_Order_Slot (Variables|/Script/Engine.ChildActorComponent|GetChildActor (Variables|Default|GetSlot1))))
  (Variables|Default|SetNPC%20for%20Payment (Variables|/Game/Others/BP_Order_Slot.BP_Order_Slot_C|GetNPC _asbp_order_slot))
  (bind _keys (Utilities|Map|Keys (Variables|/Game/NPC/BP_NPC.BP_NPC_C|GetReserve%20Products (Variables|/Game/Others/BP_Order_Slot.BP_Order_Slot_C|GetNPC _asbp_order_slot))))
  (if (Utilities|Array|ContainsItem _keys (Variables|Default|GetProduct%20For%20PIC))
    (Audio|PlaySoundatLocation "/Game/Others/Sounds/S_CashBoxPIC.S_CashBoxPIC" (Transformation|GetActorLocation) "0, 0, 0" 1.0 1.0 0.0 0 0 0 0)
    (Utilities|ChangeCash (Variables|/Game/NPC/BP_NPC.BP_NPC_C|GetReserve%20Products (Variables|/Game/Others/BP_Order_Slot.BP_Order_Slot_C|GetNPC _asbp_order_slot)))
    (Utilities|Map|Remove (Variables|/Game/NPC/BP_NPC.BP_NPC_C|GetReserve%20Products (Variables|Default|GetNPC%20for%20Payment)) (Variables|Default|GetProduct%20For%20PIC))
    (Actor|DestroyActor (Variables|Default|GetProduct%20For%20PIC))
    (if (<= (Utilities|Map|Length (Variables|/Game/NPC/BP_NPC.BP_NPC_C|GetReserve%20Products (Variables|Default|GetNPC%20for%20Payment))) 0)
      (AI|Components|Blackboard|SetValueasBool (AI|GetBlackboard (Variables|Default|GetNPC%20for%20Payment)) (Utilities|Name|MakeLiteralName "PaymentPass") true)
      (Utilities|Map|Clear (Variables|/Game/NPC/BP_NPC.BP_NPC_C|GetTakedProduct-Price (Variables|Default|GetNPC%20for%20Payment))))))

(event EventBeginPlay
  (Utilities|Array|Add (Variables|Default|GetOrder) (Variables|Default|GetSlot1))
  (Utilities|Array|Add (Variables|Default|GetOrder) (Variables|Default|GetSlot2))
  (Utilities|Array|Add (Variables|Default|GetOrder) (Variables|Default|GetSlot3)))

(event Collision|EventActorBeginOverlap
  (params (OtherActor :type Actor%20Object%20Reference)))

(event EventTick
  (params (DeltaSeconds :type Float%20%28single-precision%29)))

(fn ConstructionScript)
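; BP_Gate is a trigger that moves the products an NPC has taken to an exit spawn point when that NPC enters its box.
; It caches the first BP_ExitSpawn found at BeginPlay.
; On overlap, it loops over the NPC's TakedProductPrice map, spawning each item's class at that point.
; Each BP_DefaultStaff copy receives the mapped price before the original actor is destroyed.
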(event OnComponentBeginOverlap(Box)
  (params (OverlappedComponent :type Primitive%20Component%20Object%20Reference) (OtherActor :type Actor%20Object%20Reference) (OtherComp :type Primitive%20Component%20Object%20Reference) (OtherBodyIndex :type Integer) (bFromSweep :type Boolean) (SweepResult :type Hit%20Result%20Structure%20%28by%20ref%29))
  (bind _asbp_npc (Utilities|Casting|CastToBP_NPC OtherActor))
  (bind _keys (Utilities|Map|Keys (Variables|/Game/NPC/BP_NPC.BP_NPC_C|GetTakedProduct-Price _asbp_npc)))
  (for _array_element _keys
    (bind _returnvalue (Game|SpawnActorfromClass (Utilities|GetClass _array_element) (Math|Transform|MakeTransform (Transformation|GetWorldLocation (Variables|/Game/_AFlaot/Art/Level/BP_Products/Spawn/BP_ExitSpawn.BP_ExitSpawn_C|GetSpawnPoint (Variables|Default|GetExitSpawn))) "0, 0, 0" "1.000000,1.000000,1.000000") "Undefined" "MultiplyWithRoot" 0 0))
    (bind _asbp_default_staff (Utilities|Casting|CastToBP_DefaultStaff _returnvalue))
    (Variables|/Game/Others/Staff/BP_DefaultStaff.BP_DefaultStaff_C|SetPrice _asbp_default_staff (.Value (Utilities|Map|Find (Variables|/Game/NPC/BP_NPC.BP_NPC_C|GetTakedProduct-Price _asbp_npc) _array_element)))
    (Actor|DestroyActor _array_element)))

(event EventBeginPlay
  (bind _outactors (Actor|GetAllActorsOfClass "/Game/_AFlaot/Art/Level/BP_Products/Spawn/BP_ExitSpawn.BP_ExitSpawn_C"))
  (Variables|Default|SetExitSpawn (Utilities|Array|Get(acopy) _outactors)))

(fn ConstructionScript)
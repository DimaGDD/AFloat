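; BP_Apple is a breakable apple prop whose Price drops when it takes hard impacts.
; On Hit it estimates impact force as the hit component's velocity magnitude times its mass.
; Impacts above MinDamageStage subtract a scaled share of that force from Price, and the actor destroys itself when Price reaches zero.
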(event Collision|EventHit
  (params (MyComp :type Primitive%20Component%20Object%20Reference) (Other :type Actor%20Object%20Reference) (OtherComp :type Primitive%20Component%20Object%20Reference) (bSelfMoved :type Boolean) (HitLocation :type Vector :default "0, 0, 0") (HitNormal :type Vector :default "0, 0, 0") (NormalImpulse :type Vector :default "0, 0, 0") (Hit :type Hit%20Result%20Structure%20%28by%20ref%29))
  (Variables|Default|SetForceHit (* (Math|Vector|VectorLength (Transformation|GetComponentVelocity MyComp)) (Physics|GetMass MyComp)))
  (if (> (Variables|Default|GetForceHit) (Variables|Default|GetMinDamageStage))
    (Variables|Default|SetPrice (- (Variables|Default|GetPrice) (* (Variables|Default|GetForceHit) 0.05)))
    (if (<= (Variables|Default|GetPrice) 0.0)
      (Actor|DestroyActor))))

(fn ConstructionScript)
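; BP_Apple is an interactable apple that loses value when it takes hard impacts.
; On Hit, it multiplies component speed by mass and, above MinDamageStage, subtracts a fraction of that force from Price.
; A damaging hit shows the hint and enables CanPressF, which switches off after a short delay while the hint stays set.
; The apple destroys itself once Price reaches zero or below.
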(event Collision|EventHit
  (params (MyComp :type Primitive%20Component%20Object%20Reference) (Other :type Actor%20Object%20Reference) (OtherComp :type Primitive%20Component%20Object%20Reference) (bSelfMoved :type Boolean) (HitLocation :type Vector :default "0, 0, 0") (HitNormal :type Vector :default "0, 0, 0") (NormalImpulse :type Vector :default "0, 0, 0") (Hit :type Hit%20Result%20Structure%20%28by%20ref%29))
  (Variables|Default|SetForce%20Hit (* (Math|Vector|VectorLength (Transformation|GetComponentVelocity MyComp)) (Physics|GetMass MyComp)))
  (if (> (Variables|Default|GetForce%20Hit) (Variables|Default|GetMin%20Damage%20Stage))
    (Variables|Default|SetPrice (- (Variables|Default|GetPrice) (* (Variables|Default|GetForce%20Hit) 0.05)))
    (Variables|Default|SetHintVisible true)
    (Variables|Default|SetCanPressF true)
    (Utilities|FlowControl|Sequence
      (:then_0
        (if (<= (Variables|Default|GetPrice) 0.0)
          (Actor|DestroyActor)))
      (:then_1
        (Utilities|FlowControl|Delay 0.5)
        (Variables|Default|SetCanPressF false)))))

(event EventBeginPlay
  (Variables|Default|SetHintVisible false)
  (Variables|Default|SetCanPressF false))

(fn ConstructionScript
  (|CallParentFunction))
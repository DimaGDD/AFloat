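; BP_Spawner is an actor that spawns BP_NPC at its own transform to populate a shop up to MaxNPCInShop.
; A looping timer started on BeginPlay fires every three seconds and counts all BP_NPC actors in the world.
; Below the limit, it waits TimeBetweenSpawn, spawns one with collision adjustment, then randomizes the next wait.
; The limit is not rechecked after the delay.
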(event Custom|Spawn%20NPC
  (bind _outactors (Actor|GetAllActorsOfClass "/Game/NPC/BP_NPC.BP_NPC_C"))
  (if (< (Utilities|Array|Length _outactors) (Variables|Default|GetMax%20NPC%20in%20shop))
    (Utilities|FlowControl|Delay (Variables|Default|GetTime%20between%20spawn))
    (Game|SpawnActorfromClass "/Game/NPC/BP_NPC.BP_NPC_C" (Transformation|GetActorTransform) "AdjustIfPossibleButAlwaysSpawn" "MultiplyWithRoot" 0 0)
    (Variables|Default|SetTime%20between%20spawn (Math|Random|RandomFloatinRange 2.0 1e+01))))

(event EventBeginPlay
  (Utilities|Time|SetTimerbyEvent (delegate Custom|Spawn%20NPC) 3.0 true))

(event Collision|EventActorBeginOverlap
  (params (OtherActor :type Actor%20Object%20Reference)))

(event EventTick
  (params (DeltaSeconds :type Float%20%28single-precision%29)))

(fn ConstructionScript)
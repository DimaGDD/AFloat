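; NPC Blueprint for a shopper that gets a random appearance and shopping list on spawn.
; BeginPlay picks a random skeletal mesh and stores the first BP_XZ actor in the Blackboard's DeathPoint key.
; A delayed loop fills the ShoppingList map from PosipleStaph using a random item budget.
; Random picks re-roll at each use, and the repeat-item branch raises the remaining budget instead of lowering it.
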(event EventBeginPlay
  (bind _posiple_staph (Variables|Default|GetPosiple%20Staph))
  (bind _variablemesh (Variables|Default|GetVariableMesh))
  (bind _shopping_list (Variables|Default|GetShopping%20list))
  (bind _returnvalue (Utilities|Array|Length _posiple_staph))
  (bind _returnvalue_2 (- _returnvalue 1))
  (bind _returnvalue_3 (Math|Random|RandomIntegerinRange 0 _returnvalue_2))
  (bind _output (Utilities|Array|Get(acopy) _posiple_staph _returnvalue_3))
  (bind (_value _returnvalue_4) (Utilities|Map|Find _shopping_list _output))
  (Components|SkeletalMesh|SetSkeletalMeshAsset (Variables|Character|GetMesh) (Utilities|Array|Get(acopy) _variablemesh (Math|Random|RandomIntegerinRange 0 (- (Utilities|Array|Length _variablemesh) 1))))
  (bind _returnvalue_5 (Actor|GetActorOfClass "/Game/Others/BP_XZ.BP_XZ_C"))
  (AI|Components|Blackboard|SetValueasObject (AI|GetBlackboard 0) (Utilities|Name|MakeLiteralName "DeathPoint") _returnvalue_5)
  (bind _output_get (Variables|Default|SetMax%20Count%20Products (Math|Random|RandomIntegerinRange 0 5)))
  (while (> _output_get 0)
    (if _returnvalue_4
      (Utilities|Map|Remove _shopping_list _output)
      (Utilities|Map|Add _shopping_list _output (+ _value 1))
      (Variables|Default|SetMax%20Count%20Products (- (Variables|Default|GetMax%20Count%20Products) -1))
      (Utilities|FlowControl|Delay 0.1)
      (else
        (Utilities|Map|Add _shopping_list _output (Math|Random|RandomIntegerinRange 1 (Variables|Default|GetMax%20Count%20Products)))
        (Variables|Default|SetMax%20Count%20Products (- (Variables|Default|GetMax%20Count%20Products) (Math|Random|RandomIntegerinRange 1 (Variables|Default|GetMax%20Count%20Products))))
        (Utilities|FlowControl|Delay 0.1)))))

(event Collision|EventActorBeginOverlap
  (params (OtherActor :type Actor%20Object%20Reference)))

(event EventTick
  (params (DeltaSeconds :type Float%20%28single-precision%29)))

(fn ConstructionScript)